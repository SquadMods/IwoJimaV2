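; Frag-round cannon weapon Blueprint for a Squad emplacement, handling the cosmetic side of aiming down sights.
; On zoom it caches the seat's controller and HUD, shows the reticle overlay, quarters the user's FOV on the SPG-9 tripod scope pawn's first-person camera, and plays a timeline.
; Zooming out reverses this, as does unpossessing the owner pawn through a delegate bound one second after BeginPlay.
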(event Custom|CPossessed)

(event Custom|RemoveADS
  ;[0 0 0] ADS, change FOV and apply post processing
  (Variables|Default|GetLast%20HUD
    (:then
      (Class|SQHUD|VehicleRemoveOverlay (stale EventBlueprintonZoom _assqhud) 0)
      (bind _asbp_emplaced_spg9_tripod_scope (Utilities|Casting|CastToBP_EmplacedSPG9_TripodScope (Pawn|GetControlledPawn (Variables|Default|GetLast%20PC))))
      (Camera|SetFieldOfView (Variables|/Script/Squad.SQDeployableVehicle|GetCamera1pComponent _asbp_emplaced_spg9_tripod_scope) (Variables|/Script/Squad.SQGameUserSettings|GetFOV (Class|SQBlueprintLibrary|GetSquadGameUserSettings)))
      (Timeline|Timeline_0 Stop))
    (:else)))

(event Custom|CUnpossessed
  (CallFunction|RemoveADS))

(event EventBeginPlay
  (Utilities|FlowControl|Delay 1.0)
  (bind _assqpawn (Utilities|Casting|CastToSQPawn (Class|SQEquipableItem|GetOwnerPawn)))
  (EventDispatchers|BindEventtoOnPawnPossessedEvent _assqpawn (delegate Custom|CPossessed))
  (EventDispatchers|BindEventtoOnPawnUnPossessedEvent _assqpawn (delegate Custom|CUnpossessed)))

(event EventBlueprintonZoom
  (params (bNewZoom :type Boolean))
  (bind _returnvalue (Class|SQBlueprintLibrary|GetSquadGameUserSettings))
  (bind _returnvalue_2 (Class|SQVehicleWeapon|GetOwnerSeat))
  (bind _reticleclass (Variables|Default|GetReticleClass))
  (bind _returnvalue_3 (Pawn|GetController _returnvalue_2))
  (bind _fov (Variables|/Script/Squad.SQGameUserSettings|GetFOV _returnvalue))
  ;[0 0 0] ADS, change FOV and apply post processing
  (|CallParentFunction bNewZoom)
  (Networking|CanExecuteCosmeticEvents
    (:True
      (Variables|Default|SetLast%20PC _returnvalue_3)
      (bind _assqplayer_controller (Utilities|Casting|CastToSQPlayerController _returnvalue_3))
      (bind _assqhud (Utilities|Casting|CastToSQHUD (HUD|GetHUD _assqplayer_controller)))
      (Variables|Default|SetLast%20HUD _assqhud)
      (if bNewZoom
        (if (Utilities|IsValidClass _reticleclass)
          (Class|SQHUD|VehicleCreateOverlay _assqhud _reticleclass)
          (bind _asbp_emplaced_spg9_tripod_scope (Utilities|Casting|CastToBP_EmplacedSPG9_TripodScope (Pawn|GetControlledPawn (Variables|Default|GetLast%20PC))))
          (Camera|SetFieldOfView (Variables|/Script/Squad.SQDeployableVehicle|GetCamera1pComponent _asbp_emplaced_spg9_tripod_scope) (/ _fov 4.0))
          (Timeline|Timeline_0 Play)
          (else
            (Class|SQHUD|VehicleRemoveOverlay _assqhud 0 :!label _label)
            (bind _asbp_emplaced_spg9_tripod_scope_2 (Utilities|Casting|CastToBP_EmplacedSPG9_TripodScope (Pawn|GetControlledPawn (Variables|Default|GetLast%20PC))))
            (Camera|SetFieldOfView (Variables|/Script/Squad.SQDeployableVehicle|GetCamera1pComponent _asbp_emplaced_spg9_tripod_scope_2) _fov)
            (Timeline|Timeline_0 Stop)))
        (else
          (goto _label))))))

(fn ConstructionScript
  (|CallParentFunction))