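; MovingFlag_BP is a capturable flag that moves and swaps between US and Militia materials when its trigger box is occupied.
; Overlapping the box plays the FlagMovement timeline, which drives the flag's relative location, and leaving reverses it.
; Timeline event tracks toggle the material and IsUSCaptured, play a flag sound, and stop the timeline at the capture point.
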(event OnComponentEndOverlap(TriggerBox)
  (params (OverlappedComponent :type Primitive%20Component%20Object%20Reference) (OtherActor :type Actor%20Object%20Reference) (OtherComp :type Primitive%20Component%20Object%20Reference) (OtherBodyIndex :type Integer))
  (bind _flaglocation (Timeline|FlagMovement Reverse)
    (:Update
      (Transformation|SetRelativeLocation (Variables|Default|GetFlag) _flaglocation false false))
    (:MaterialChange
      (if (Variables|Default|GetisUSCaptured)
        (CallFunction|FlagMaterialMIL)
        (else
          (CallFunction|FlagMaterialUS))))
    (:FlagCaptured
      (CallFunction|FlagCaptured))
    (:Audio
      (Audio|PlaySoundatLocation "/IwoJimav2/IwoJima/IwoJimaV2_sharedassets/Ambient/Flageffect.Flageffect" (Variables|Default|GetInitialFlagLocation) "0, 0, 0" 0.75 1.0 0.0 0 "/Game/Audio/Concurrency/AmbientConcurrency.AmbientConcurrency"))))

(event OnComponentBeginOverlap(TriggerBox)
  (params (OverlappedComponent :type Primitive%20Component%20Object%20Reference) (OtherActor :type Actor%20Object%20Reference) (OtherComp :type Primitive%20Component%20Object%20Reference) (OtherBodyIndex :type Integer) (bFromSweep :type Boolean) (SweepResult :type Hit%20Result%20Structure%20%28by%20ref%29))
  (bind _flaglocation (Timeline|FlagMovement Play)
    (:Update
      (Transformation|SetRelativeLocation (Variables|Default|GetFlag) _flaglocation false false))
    (:MaterialChange
      (if (Variables|Default|GetisUSCaptured)
        (CallFunction|FlagMaterialMIL)
        (else
          (CallFunction|FlagMaterialUS))))
    (:FlagCaptured
      (CallFunction|FlagCaptured))
    (:Audio
      (Audio|PlaySoundatLocation "/IwoJimav2/IwoJima/IwoJimaV2_sharedassets/Ambient/Flageffect.Flageffect" (Variables|Default|GetInitialFlagLocation) "0, 0, 0" 0.75 1.0 0.0 0 "/Game/Audio/Concurrency/AmbientConcurrency.AmbientConcurrency"))))

(event Custom|FlagCaptured
  (bind _flaglocation (Timeline|FlagMovement Stop)
    (:Update
      (Transformation|SetRelativeLocation (Variables|Default|GetFlag) _flaglocation false false))
    (:MaterialChange
      (if (Variables|Default|GetisUSCaptured)
        (CallFunction|FlagMaterialMIL)
        (else
          (CallFunction|FlagMaterialUS))))
    (:FlagCaptured
      (CallFunction|FlagCaptured))
    (:Audio
      (Audio|PlaySoundatLocation "/IwoJimav2/IwoJima/IwoJimaV2_sharedassets/Ambient/Flageffect.Flageffect" (Variables|Default|GetInitialFlagLocation) "0, 0, 0" 0.75 1.0 0.0 0 "/Game/Audio/Concurrency/AmbientConcurrency.AmbientConcurrency"))))

(fn ConstructionScript)

(fn FlagMaterialUS
  (Rendering|Material|SetMaterial (Variables|Default|GetFlag) 1 "/Game/Maps/Jensens_Range/Assets/Flags/MI_Flag_USA.MI_Flag_USA")
  (Variables|Default|SetisUSCaptured true))

(fn FlagMaterialMIL
  (Rendering|Material|SetMaterial (Variables|Default|GetFlag) 1 "/Game/Maps/Jensens_Range/Assets/Flags/MI_Flag_Militia.MI_Flag_Militia")
  (Variables|Default|SetisUSCaptured false))