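; BP_Campfire_IWo is a placeable campfire prop for the Iwo Jima map that can be lit or unlit through a Burning flag.
; The construction script applies a cull distance to the mesh, sets an Emissive parameter on a dynamic material to match the state, and adds a particle system with the same cull distance when burning.
; On BeginPlay, a burning campfire activates its audio component.
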(event EventBeginPlay
  (if (Variables|Default|GetBurning?)
    (Components|Activation|Activate (Variables|Default|GetAudio) false)))

(fn ConstructionScript
  (Class|PrimitiveComponent|SetCullDistance (Variables|Default|GetStaticMesh) (Variables|Default|GetCullDistance))
  (if (Variables|Default|GetBurning?)
    (bind _returnvalue (Rendering|Material|CreateDynamicMaterialInstance (Variables|Default|GetStaticMesh) 0 0 :!class /Script/Engine.PrimitiveComponent))
    (Rendering|Material|SetScalarParameterValue _returnvalue "Emissive" 1.0 :!class /Script/Engine.MaterialInstanceDynamic)
    (bind _returnvalue_2 (AddComponent|AddParticleSystemComponent false))
    (Class|PrimitiveComponent|SetCullDistance _returnvalue_2 (Variables|Default|GetCullDistance))
    (else
      (bind _returnvalue_3 (Rendering|Material|CreateDynamicMaterialInstance (Variables|Default|GetStaticMesh) 0 0 :!class /Script/Engine.PrimitiveComponent))
      (Rendering|Material|SetScalarParameterValue _returnvalue_3 "Emissive" 0.0 :!class /Script/Engine.MaterialInstanceDynamic))))